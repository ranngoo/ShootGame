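; Enemy charger pawn that chases the player and detonates on contact, costing the player 25 HP.
; PawnSensing spots a FirstPersonCharacter, turns the point light pink-red and sends the enemy after it with AI MoveTo.
; Overlapping its capsule with the player destroys the enemy and subtracts the damage directly from PlayerHP.
; An unconnected node for setting the light green is left unused.
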(event `self.CapsuleComponent.OnComponentBeginOverlap`
  (params (OverlappedComponent :type "PrimitiveComponent Object Reference") (OtherActor :type "Actor Object Reference") (OtherComp :type "PrimitiveComponent Object Reference") (OtherBodyIndex :type Integer) (bFromSweep :type Boolean) (SweepResult :type "HitResult Structure (by ref)"))
  (bind _asfirst_person_character (cast `/Game/FirstPersonBP/Blueprints/FirstPersonCharacter` OtherActor))
  (`|ExecutionSequence`
    (:`then_0`
      (bind _asenemycharger (cast `/Game/Blueprints/enemycharger` self))
      (`self.K2_DestroyActor` _asenemycharger))
    (:`then_1`
      (set `/Game/FirstPersonBP/Blueprints/FirstPersonCharacter.playerHP` (- (`/Game/FirstPersonBP/Blueprints/FirstPersonCharacter.playerHP` _asfirst_person_character) 25.0) _asfirst_person_character))))

(event `self.PawnSensing.OnSeePawn`
  (params (Pawn :type "Pawn Object Reference"))
  (bind _asfirst_person_character (cast `/Game/FirstPersonBP/Blueprints/FirstPersonCharacter` Pawn))
  (`|ExecutionSequence`
    (:`then_0`
      (`LightComponent.SetLightColor` (`self.PointLight`) (struct :`R` 1.0 :`G` 0.012008 :`B` 0.422747 :`A` 1.0) true))
    (:`then_1`
      (`|AIMoveTo` self (0.0 0.0 0.0) _asfirst_person_character))))

(fn `UserConstructionScript`)