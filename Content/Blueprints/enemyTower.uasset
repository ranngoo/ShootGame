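; Enemy tower actor that damages the first-person player on contact and destroys itself.
; A capsule overlap with the FirstPersonCharacter destroys the tower, then subtracts a fixed amount from that character's PlayerHP.
; Tick also polls the tower's own HPet health value and destroys the actor once it reaches zero or below; nothing in this graph lowers that value.
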(event `self.ReceiveTick`
  (params (DeltaSeconds :type "Float (single-precision)"))
  (if (<= (`self.HPet`) 0.0)
    (`self.K2_DestroyActor`)))

(event `self.CapsuleComponent.OnComponentBeginOverlap`
  (params (OverlappedComponent :type "PrimitiveComponent Object Reference") (OtherActor :type "Actor Object Reference") (OtherComp :type "PrimitiveComponent Object Reference") (OtherBodyIndex :type Integer) (bFromSweep :type Boolean) (SweepResult :type "HitResult Structure (by ref)"))
  (bind _asfirst_person_character (cast `/Game/FirstPersonBP/Blueprints/FirstPersonCharacter` OtherActor))
  (`|ExecutionSequence`
    (:`then_0`
      (bind _asenemy_tower (cast `/Game/Blueprints/enemyTower` self))
      (`self.K2_DestroyActor` _asenemy_tower))
    (:`then_1`
      (set `/Game/FirstPersonBP/Blueprints/FirstPersonCharacter.playerHP` (- (`/Game/FirstPersonBP/Blueprints/FirstPersonCharacter.playerHP` _asfirst_person_character) 25.0) _asfirst_person_character))))

(fn `UserConstructionScript`)